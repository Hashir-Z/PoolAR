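; Billiard game Blueprint that lets the AI choose, aim and take shots, respawns the pocketed white ball and signals when no balls remain.
; Target search picks a ball with a clear path to a hole, optionally within an index range, else a random one, leaving the 8-ball last.
; Distance from white ball to target location sets force.
; Per-frame Delay loops animate cue draw and strike, then fire the shot with the given accuracy.
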(event Custom|StopAimByAI
  (params (Accuracy :type Float%20%28double-precision%29))
  (Variables|Default|SetStarted false)
  (Variables|Default|SetLastForce (CallFunction|ConvertFactortoForce))
  ;[1 1 1] Animate Cue hit BallWhite, when you released click.
  (if (> (Variables|Default|GetLastForce) 0.01) :!label _label
    (Utilities|FlowControl|Delay (Utilities|Time|GetWorldDeltaSeconds))
    (bind _output_get (Variables|Default|SetLastForce (Math|Float|Power (Variables|Default|GetLastForce) 3.0)))
    (CallFunction|AISetCuetoBallWhite _output_get)
    (goto _label)
    (else
      (Utilities|FlowControl|Sequence
        (:then_0
          (CallFunction|ShottoTarget Accuracy)
          (CallFunction|ResetCuetoStart))
        (:then_1
          (Variables|Default|SetLastForce 0.0)
          (Variables|AITarget|SetAITargetForce 0.0))))))

(event Custom|StartAimByAI
  (params (Accuracy :type Float%20%28double-precision%29))
  (bind (_ballactor _hitlocation _returnvalue) (CallFunction|FindBalltoShot))
  (Variables|Default|SetStarted true)
  (Variables|Default|SetFactor 0.0)
  (Utilities|FlowControl|Delay (Utilities|Time|GetWorldDeltaSeconds) :!label _label)
  (if (Variables|Default|GetStarted)
    (if (> (Variables|AITarget|GetAITargetForce) 0.0)
      (CallFunction|AISetCuetoBallWhite (CallFunction|ConvertFactortoForce))
      (if (Math|Float|NearlyEqual(Float) (CallFunction|ConvertFactortoForce) (Variables|AITarget|GetAITargetForce) 0.01)
        (CallFunction|StopAimbyAI Accuracy)
        (else
          (goto _label)))
      (else
        ;[1 1 1] Get Possible shot
        (if _returnvalue
          (CallFunction|SetAITarget _ballactor _hitlocation)
          (goto _label))))))

(event Custom|ShotToTarget
  (params (Accuracy :type Float%20%28double-precision%29))
  (bind _ball (CallFunction|GetBallWhite))
  (if (> (Variables|AITarget|GetAITargetForce) 0.0)
    (Default|ShotBalltoHole (CallFunction|GetBallWhite) (Variables|AITarget|GetAITargetShotBall) (Variables|AITarget|GetAITargetHoleLocation) Accuracy)
    (Default|PlaySound _ball "/Game/BilliardGameFramework/Sounds/Cues/Billiard_Bat_10_Cue.Billiard_Bat_10_Cue" (Collision|MakeHitResult false false 0.0 0.0 "0, 0, 0" "0, 0, 0" "0,0,1" (Variables|/Game/BilliardGameFramework/Blueprints/BP_Ball.BP_Ball_C|GetVelocityPerSecond _ball) 0 0))))

(event Custom|AddRndomBalls
  (params (BallsCount :type Integer))
  (for _index (range 1 BallsCount)
    (bind _returnvalue (AddComponent|AddChildActorComponent false (Math|Transform|MakeTransform (Math|Vector|MakeVector (Math|Random|RandomFloatinRange -6e+01 6e+01) (Math|Random|RandomFloatinRange -1.2e+02 1.2e+02) 3e+01) "0, 0, 0" "1.000000,1.000000,1.000000")))
    (Transformation|AttachComponentToComponent _returnvalue (Variables|Default|GetOthers) "None" "KeepRelative" "KeepRelative" "KeepRelative" true)
    (ChildActorComponent|SetChildActorClass _returnvalue "/Game/BilliardGameFramework/Blueprints/BP_Ball.BP_Ball_C")
    (Variables|/Game/BilliardGameFramework/Blueprints/BP_Ball.BP_Ball_C|SetBallIndex (.AsBP%20Ball (Utilities|Casting|CastToBP_Ball (Variables|/Script/Engine.ChildActorComponent|GetChildActor _returnvalue))) (Math|Random|RandomIntegerinRange 1 7))
    (Default|SetBallStaticMesh (.AsBP%20Ball (Utilities|Casting|CastToBP_Ball (Variables|/Script/Engine.ChildActorComponent|GetChildActor _returnvalue))))))

(event Custom|Call_OnBallInTheHole
  (params (BallIndex :type Integer))
  (if (Utilities|Array|IsEmpty (CallFunction|GetEnableBalls))
    (Default|CallOnNoBalltoShot)))

(event Custom|StartAimByAIWithRange
  (params (BallIndexRange :type Array%20of%20Integers) (Accuracy :type Float%20%28double-precision%29))
  (bind (_ballactor _hitlocation _returnvalue) (CallFunction|FindBalltoShotwithRange BallIndexRange))
  (if _returnvalue :!label _label
    (CallFunction|SetAITarget _ballactor _hitlocation)
    (CallFunction|StartAimbyAI Accuracy)
    (else
      (Utilities|FlowControl|Delay (Utilities|Time|GetWorldDeltaSeconds))
      (goto _label))))

(event Custom|SetAITarget
  (params (BallActor :type BP%20Ball%20Object%20Reference) (HitLocation :type Vector))
  (Variables|AITarget|SetAITargetForce (Math|Float|Min(Float) (/ (Math|Vector|Distance(Vector) HitLocation (Default|GetOrigin (CallFunction|GetBallWhite))) 2e+02) 1.0))
  (Variables|AITarget|SetAITargetHoleLocation HitLocation)
  (Variables|AITarget|SetAITargetShotBall BallActor))

(event EventBeginPlay
  (|CallParentFunction)
  (Utilities|FlowControl|Sequence
    (:then_0
      (Variables|Cache|SetCacheMovingBall (CallFunction|GetBallWhite)))
    (:then_1
      (EventDispatchers|BindEventtoOnBallintheHole (EventDispatchers|CreateEvent :!event Custom|Call_OnBallInTheHole)))))

(event Collision|EventActorBeginOverlap
  (params (OtherActor :type Actor%20Object%20Reference))
  (|CallParentFunction OtherActor) ; This node is disabled and will not be called.\nDrag off pins to build functionality.
)

(event EventTick
  (params (DeltaSeconds :type Float%20%28single-precision%29))
  (|CallParentFunction DeltaSeconds)
  (Utilities|FlowControl|Sequence
    (:then_0
      ;[1 1 1] When white ball in the hole, reset it.
      (if (not (Default|IsEnable (CallFunction|GetBallWhite)))
        (CallFunction|ResetBallWhite)))))

(fn ConstructionScript
  (|CallParentFunction))

(fn GetBall
  (params (Child%20Actor :type Child%20Actor%20Component%20Object%20Reference))
  (bind _asbp_ball (Utilities|Casting|CastToBP_Ball (Variables|/Script/Engine.ChildActorComponent|GetChildActor Child%20Actor))
    (:then
      (return _asbp_ball true))
    (:CastFailed
      (return 0 false))))

(fn GetBallWhite
  (return (.Ball (CallFunction|GetBall (Variables|Default|GetBall0-White)))))

(fn GetEnableBalls
  ;[1 1 1] Get enable balls expect white ball.
  (Utilities|FlowControl|Sequence
    (:then_0
      (LocalVariables|SetLocalSceneComponents (Components|GetChildrenComponents (Variables|Default|GetOthers) false)))
    (:then_1
      (for _array_element (LocalVariables|GetLocalSceneComponents)
        (if (.ReturnValue (Utilities|Map|Find (Variables|Cache|GetCacheBalls) _array_element)) :!label _label
          (if (Math|Boolean|ANDBoolean (Default|IsEnable (.Value (Utilities|Map|Find (Variables|Cache|GetCacheBalls) _array_element))) (!= (Variables|/Game/BilliardGameFramework/Blueprints/BP_Ball.BP_Ball_C|GetBallIndex (.Value (Utilities|Map|Find (Variables|Cache|GetCacheBalls) _array_element))) 0) (Utilities|IsValid (.Value (Utilities|Map|Find (Variables|Cache|GetCacheBalls) _array_element))))
            (if (!= (Variables|/Game/BilliardGameFramework/Blueprints/BP_Ball.BP_Ball_C|GetBallIndex (.Value (Utilities|Map|Find (Variables|Cache|GetCacheBalls) _array_element))) 8)
              (Utilities|Array|Add (LocalVariables|GetEnableBalls) (.Value (Utilities|Map|Find (Variables|Cache|GetCacheBalls) _array_element)))
              (else
                (Utilities|Array|Add (LocalVariables|GetEnableBlackBalls) (.Value (Utilities|Map|Find (Variables|Cache|GetCacheBalls) _array_element))))))
          (else
            (bind _aschild_actor_component (Utilities|Casting|CastToChildActorComponent _array_element))
            (bind _asbp_ball (Utilities|Casting|CastToBP_Ball (Variables|/Script/Engine.ChildActorComponent|GetChildActor _aschild_actor_component)))
            (Utilities|Map|Add (Variables|Cache|GetCacheBalls) _array_element _asbp_ball)
            (goto _label))))
      (if (Utilities|Array|IsEmpty (LocalVariables|GetEnableBalls))
        (return (LocalVariables|GetEnableBlackBalls))
        (else
          (return (LocalVariables|GetEnableBalls)))))))

(fn GetEnableBlackBalls
  ;[1 1 1] Get enable balls expect white ball.
  (Utilities|FlowControl|Sequence
    (:then_0
      (LocalVariables|SetLocalSceneComponents (Components|GetChildrenComponents (Variables|Default|GetOthers) false)))
    (:then_1
      (for _array_element (LocalVariables|GetLocalSceneComponents)
        (if (.ReturnValue (Utilities|Map|Find (Variables|Cache|GetCacheBalls) _array_element)) :!label _label
          (if (and (Default|IsEnable (.Value (Utilities|Map|Find (Variables|Cache|GetCacheBalls) _array_element))) (== (Variables|/Game/BilliardGameFramework/Blueprints/BP_Ball.BP_Ball_C|GetBallIndex (.Value (Utilities|Map|Find (Variables|Cache|GetCacheBalls) _array_element))) 8))
            (Utilities|Array|Add (LocalVariables|GetEnableBlackBalls) (.Value (Utilities|Map|Find (Variables|Cache|GetCacheBalls) _array_element))))
          (else
            (bind _aschild_actor_component (Utilities|Casting|CastToChildActorComponent _array_element))
            (bind _asbp_ball (Utilities|Casting|CastToBP_Ball (Variables|/Script/Engine.ChildActorComponent|GetChildActor _aschild_actor_component)))
            (Utilities|Map|Add (Variables|Cache|GetCacheBalls) _array_element _asbp_ball)
            (goto _label))))
      (return (LocalVariables|GetEnableBlackBalls)))))

(fn GetNotMovingEnableBalls
  ;[1 1 1] Get enable and not moving balls expect white ball.
  (for _array_element (CallFunction|GetEnableBalls)
    (if (< (Math|Vector|VectorLength (Variables|/Game/BilliardGameFramework/Blueprints/BP_Ball.BP_Ball_C|GetVelocityPerSecond _array_element)) 0.1)
      (Utilities|Array|Add (LocalVariables|GetEnableBalls) _array_element)))
  (return (LocalVariables|GetEnableBalls)))

(fn FindBalltoShot
  (bind _balls (CallFunction|GetEnableBalls))
  (bind (_ballactor _hitlocation _returnvalue) (CallFunction|FindBalltoShotfromOffer _balls))
  ;[1 1 1] Loop all balls and all holes find possible shot
  (return _ballactor _hitlocation _returnvalue))

(fn FindBalltoShotfromOffer
  (params (OfferBalls :type Array%20of%20BP%20Ball%20Object%20References))
  ;[1 1 1] Loop all balls and all holes find possible shot
  (LocalVariables|SetLocalBalls OfferBalls)
  (bind _array_element (Utilities|Array|ForEachLoopwithBreak (LocalVariables|GetLocalBalls))
    (:LoopBody
      (if (.ReturnValue (CallFunction|FindShotableHoleLocation _array_element))
        (return _array_element (.HitLocation (CallFunction|FindShotableHoleLocation _array_element)) true)))
    (:Completed
      (if (Utilities|Array|IsEmpty (LocalVariables|GetLocalBalls))
        (return 0 "0, 0, 0" false)
        (else
          (return (.OutItem (Utilities|Array|Random (LocalVariables|GetLocalBalls))) (Default|GetOrigin (.OutItem (Utilities|Array|Random (LocalVariables|GetLocalBalls)))) true))))))

(fn FindBalltoShotwithRange
  (params (BallIndexRange :type Array%20of%20Integers))
  ;[1 1 1] Loop all balls and all holes find possible shot
  (Utilities|FlowControl|Sequence
    (:then_0
      (Utilities|Array|Add BallIndexRange 8)
      (bind _output_get (LocalVariables|SetGotBalls (CallFunction|GetEnableBalls)))
      (for _array_element _output_get
        (if (Utilities|Array|ContainsItem BallIndexRange (Variables|/Game/BilliardGameFramework/Blueprints/BP_Ball.BP_Ball_C|GetBallIndex _array_element))
          (Utilities|Array|Add (LocalVariables|GetLocalBalls) _array_element))))
    (:then_1
      (if (Utilities|Array|IsEmpty (LocalVariables|GetLocalBalls))
        (LocalVariables|SetLocalBalls (CallFunction|GetEnableBlackBalls))))
    (:then_2
      (return (.BallActor (CallFunction|FindBalltoShotfromOffer (LocalVariables|GetLocalBalls))) (.HitLocation (CallFunction|FindBalltoShotfromOffer (LocalVariables|GetLocalBalls))) (.ReturnValue (CallFunction|FindBalltoShotfromOffer (LocalVariables|GetLocalBalls)))))))

(fn FindShotableHoleLocation
  (params (BallActor :type BP%20Ball%20Object%20Reference))
  ;[1 1 1] Loop all holes to test the ball has clean shot.
  (Utilities|IsValid BallActor
    (:Is%20Valid
      (Utilities|FlowControl|Sequence
        (:then_0
          (for _array_element (Components|GetChildrenComponents (Variables|Default|GetHoles) false)
            (Utilities|Array|Add (LocalVariables|GetLocations) (Transformation|GetWorldLocation _array_element))))
        (:then_1
          (bind _array_element_2 (Utilities|Array|ForEachLoopwithBreak (LocalVariables|GetLocations))
            (:LoopBody
              (if (Default|IsPossibleBalltoHole (CallFunction|GetBallWhite) BallActor _array_element_2)
                (return _array_element_2 (Default|IsPossibleBalltoHole (CallFunction|GetBallWhite) BallActor _array_element_2))))))))
    (:Is%20Not%20Valid
      (return "0, 0, 0" false))))

(fn AIIsReadytoStartAim
  ;[1 1 1] When white ball isn't moving and cue aniamtion stops, start AI aim and shot
  (if (Math|Boolean|ANDBoolean (not (Variables|Default|GetStarted)) (== (Variables|Default|GetLastForce) 0.0) (< (Math|Vector|VectorLength (Variables|/Game/BilliardGameFramework/Blueprints/BP_Ball.BP_Ball_C|GetVelocityPerSecond (CallFunction|GetBallWhite))) 0.1) (< (Math|Vector|VectorLength (Variables|/Game/BilliardGameFramework/Blueprints/BP_Ball.BP_Ball_C|GetVelocityPerSecond (Variables|Cache|GetCacheMovingBall))) 0.1))
    (bind _output_get (LocalVariables|SetStore (CallFunction|GetEnableBalls)))
    (if (Utilities|Array|IsNotEmpty _output_get)
      (for _array_element (LocalVariables|GetStore)
        (if (not (< (Math|Vector|VectorLength (Variables|/Game/BilliardGameFramework/Blueprints/BP_Ball.BP_Ball_C|GetVelocityPerSecond _array_element)) 0.1))
          (Variables|Cache|SetCacheMovingBall _array_element)
          (return false)))
      (return true)
      (else
        (return false)))
    (else
      (return false))))

(fn AISetCuetoBallWhite
  (params (Force :type Float%20%28double-precision%29))
  ;[1 1 1] Set cue target white ball with aim direction
  (Utilities|IsValid (Variables|AITarget|GetAITargetShotBall)
    (:Is%20Valid
      (CallFunction|SetCuetoBallWhite Force (- (Default|CalcShotBallHitLocation (CallFunction|GetBallWhite) (Variables|AITarget|GetAITargetShotBall) (Variables|AITarget|GetAITargetHoleLocation)) (Default|GetOrigin (CallFunction|GetBallWhite))) false))))